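; Player character Blueprint that handles the player's HUD crosshair and feedback when health changes.
; On begin play it creates a Crosshair widget and adds it to the viewport.
; The HealthComponent's health change event plays a camera shake at the camera and adds a new HurtScreen widget on damage.
; Otherwise it prints a debug "Healed!" message with the delta.
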(event OnHealthChanged(HealthComponent)
  (params (HealthComp :type STS%20Health%20Component%20Object%20Reference) (Health :type Float%20%28single-precision%29) (HealthDelta :type Float%20%28single-precision%29) (DamageType :type Damage%20Type%20Object%20Reference) (InstigatedBy :type Controller%20Object%20Reference) (DamageCauser :type Actor%20Object%20Reference))
  (if (< HealthDelta 0.0)
    (Camera|PlayWorldCameraShake "/Game/FX/HitCameraShake.HitCameraShake_C" (Transformation|GetWorldLocation (Variables|Default|GetCameraComponent)) 0.0 5e+01)
    (bind _returnvalue (UserInterface|CreateWidget "/Game/FX/HurtScreen.HurtScreen_C"))
    (UserInterface|Viewport|AddtoViewport _returnvalue 0)
    (else
      (Development|PrintString (Utilities|String|Append "Healed! " (Utilities|String|ToString(Float) HealthDelta))))))

(event EventBeginPlay
  (bind _returnvalue (UserInterface|CreateWidget "/Game/FX/Crosshair.Crosshair_C"))
  (UserInterface|Viewport|AddtoViewport _returnvalue 0))

(fn ConstructionScript)